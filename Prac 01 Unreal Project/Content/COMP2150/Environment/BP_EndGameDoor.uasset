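; End-game door actor that tracks the key count in BP_2150GameMode and opens once three keys are held.
; Tick polls the count, turning the matching key slot green, and at three also lights the frame and calls MoveDoor.
; MoveDoor eases the two leaves toward mirrored relative targets with a delta-time-scaled lerp from their current positions.
; Any overlap on the Exit component loads LevelToLoad, with no key check.
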(event `self.ReceiveTick`
  (params (DeltaSeconds :type "Float (single-precision)"))
  (bind _keys (`/Game/COMP2150/Core/MainGame/BP_2150GameMode.Keys` (`self.GameMode`)))
  (if (== _keys 1)
    (`PrimitiveComponent.SetMaterial` (`self.KeySlot1`) 0 "/Game/COMP2150/Generic/M_GlowGreen.M_GlowGreen")
    (elif (== _keys 2)
      (`PrimitiveComponent.SetMaterial` (`self.KeySlot2`) 0 "/Game/COMP2150/Generic/M_GlowGreen.M_GlowGreen")
      (elif (== _keys 3)
        (`self.MoveDoor`)
        (`PrimitiveComponent.SetMaterial` (`self.KeySlot3`) 0 "/Game/COMP2150/Generic/M_GlowGreen.M_GlowGreen")
        (`PrimitiveComponent.SetMaterial` (`self.DoorFrame`) 0 "/Game/COMP2150/Generic/M_GlowGreen.M_GlowGreen")))))

(event `MoveDoor`
  (`SceneComponent.K2_SetRelativeLocation` (`self.LeftDoor`) (`KismetMathLibrary.VLerp` (.location (`SceneComponent.GetRelativeTransform` (`self.LeftDoor`))) (`self.TargetLocation`) (* (`self.DoorSpeed`) (`GameplayStatics.GetWorldDeltaSeconds`))) false false)
  (`SceneComponent.K2_SetRelativeLocation` (`self.RightDoor`) (`KismetMathLibrary.VLerp` (.location (`SceneComponent.GetRelativeTransform` (`self.RightDoor`))) (* (`self.TargetLocation`) (0.0 -1.0 0.0)) (* (`self.DoorSpeed`) (`GameplayStatics.GetWorldDeltaSeconds`))) false false))

(event `self.ReceiveBeginPlay`
  (bind _asbp_2150game_mode (cast `/Game/COMP2150/Core/MainGame/BP_2150GameMode` (`GameplayStatics.GetGameMode`)))
  (set `self.GameMode` _asbp_2150game_mode))

(event `self.Exit.OnComponentBeginOverlap`
  (params (OverlappedComponent :type "PrimitiveComponent Object Reference") (OtherActor :type "Actor Object Reference") (OtherComp :type "PrimitiveComponent Object Reference") (OtherBodyIndex :type Integer) (bFromSweep :type Boolean) (SweepResult :type "HitResult Structure (by ref)"))
  (`GameplayStatics.OpenLevelBySoftObjectPtr` (`.WorldAsset` (break `SoftWorldReference` (`self.LevelToLoad`)))))

(fn `UserConstructionScript`)