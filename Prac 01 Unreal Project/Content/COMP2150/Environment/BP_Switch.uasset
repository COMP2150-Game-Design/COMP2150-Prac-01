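; BP_Switch is a one-shot switch that fires when hit by a "Projectile"-tagged actor or through ClickTriggered.
; It calls Triggered on the Receiver actor's BP_SwitchReceiverComponent, latches On, and requests a brief green glow.
; Tick sets orange or red from the highlight flag every frame, overriding that green.
; The construction script draws a debug line to the Receiver to show the link.
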(event `ClickTriggered`
  (if true
    (if (not (`self.On`))
      (`/Game/COMP2150/Environment/BP_SwitchReceiverComponent.Triggered` (`self.GetComponentByClass` (`self.Receiver`) "/Game/COMP2150/Environment/BP_SwitchReceiverComponent.BP_SwitchReceiverComponent_C") :!label _label)
      (set `self.On` true)
      (`PrimitiveComponent.SetMaterial` (`self.Mesh`) 0 "/Game/COMP2150/Generic/M_GlowGreen.M_GlowGreen")
      (`KismetSystemLibrary.Delay` 0.5)
      (`PrimitiveComponent.SetMaterial` (`self.Mesh`) 0 "/Game/COMP2150/Generic/M_GlowRed.M_GlowRed"))
    (else
      (goto _label))))

(event `self.ReceiveHit`
  (params (MyComp :type "PrimitiveComponent Object Reference") (Other :type "Actor Object Reference") (OtherComp :type "PrimitiveComponent Object Reference") (bSelfMoved :type Boolean) (HitLocation :type "Vector Structure") (HitNormal :type "Vector Structure") (NormalImpulse :type "Vector Structure") (Hit :type "HitResult Structure (by ref)"))
  (if (`self.ActorHasTag` Other "Projectile")
    (`self.ClickTriggered`)))

(event `self.ReceiveTick`
  (params (DeltaSeconds :type "Float (single-precision)"))
  (bind _mesh (`self.Mesh`))
  (if (`self.Highlighted`)
    (`PrimitiveComponent.SetMaterial` _mesh 0 "/Game/COMP2150/Generic/M_GlowOrange.M_GlowOrange")
    (else
      (`PrimitiveComponent.SetMaterial` _mesh 0 "/Game/COMP2150/Generic/M_GlowRed.M_GlowRed"))))

(event `SetHighlight`
  (params (Input :type Boolean))
  (set `self.Highlighted` Input))

(fn `UserConstructionScript`
  (`KismetSystemLibrary.FlushPersistentDebugLines`)
  (`KismetSystemLibrary.DrawDebugLine` (`self.K2_GetActorLocation`) (`self.K2_GetActorLocation` (`self.Receiver`)) (struct :`R` 0.400182 :`G` 0.275666 :`B` 1.0 :`A` 1.0) 900.0 5.0))