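; BP_Door is a sliding double door that opens and closes according to the state of its switch receiver.
; BeginPlay caches BPSwitchReceiver, and each Tick copies its On flag into Open to choose the open or closed target offset.
; MoveDoor lerps both panels' relative locations toward that target every frame, mirroring the left one on Y, with delta-scaled DoorSpeed giving an eased slide.
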(event `self.ReceiveBeginPlay`
  (set `self.SwitchReceiver` (`self.BP_SwitchReceiver`)))

(event `self.ReceiveTick`
  (params (DeltaSeconds :type "Float (single-precision)"))
  (if (`KismetSystemLibrary.IsValid` (`self.SwitchReceiver`))
    (set `self.Open` (`/Game/COMP2150/Environment/BP_SwitchReceiverComponent.On` (`self.SwitchReceiver`))))
  (`self.OpenCheck`)
  (`self.MoveDoor`))

(event `OpenCheck`
  (if (`self.Open`)
    (set `self.TargetLocation` (0.0 210.0 0.0))
    (else
      (set `self.TargetLocation` (0.0 0.0 0.0)))))

(event `MoveDoor`
  (`SceneComponent.K2_SetRelativeLocation` (`self.LeftDoor`) (`KismetMathLibrary.VLerp` (.location (`SceneComponent.GetRelativeTransform` (`self.LeftDoor`))) (* (`self.TargetLocation`) (0.0 -1.0 0.0)) (* (`self.DoorSpeed`) (`GameplayStatics.GetWorldDeltaSeconds`))) false false)
  (`SceneComponent.K2_SetRelativeLocation` (`self.RightDoor`) (`KismetMathLibrary.VLerp` (.location (`SceneComponent.GetRelativeTransform` (`self.RightDoor`))) (`self.TargetLocation`) (* (`self.DoorSpeed`) (`GameplayStatics.GetWorldDeltaSeconds`))) false false))

(fn `UserConstructionScript`)