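; Game mode for the COMP2150 game, owning the Sinead player's health, mana, keys, ability unlocks and respawn point.
; BeginPlay creates the gameplay UI, caches the player and records the spawn point; stat and key changes update that UI directly.
; A Delay on Tick throttles mana regen, which also refreshes Blink and Shield availability from cost and unlock state.
; Zero health teleports the player to spawn with full stats; collected keys fire GameStateChange.
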(event `self.ReceiveTick`
  (params (DeltaSeconds :type "Float (single-precision)"))
  (`KismetSystemLibrary.Delay` 0.2)
  (`self.RestoreMana`))

(event `self.ReceiveBeginPlay`
  ; Build UI and find Player
  (bind _returnvalue (`|CreateWidget` "/Game/COMP2150/UI/UI_2150Gameplay.UI_2150Gameplay_C" (`GameplayStatics.GetPlayerController` 0)))
  (bind _output_get (set `self.UI` _returnvalue))
  (`UserWidget.AddToViewport` _output_get 0)
  (bind _asbp_sinead (cast `/Game/COMP2150/Core/MainGame/BP_Sinead` (`GameplayStatics.GetPlayerPawn` 0)))
  (bind _output_get_2 (set `self.Player` _asbp_sinead))
  (`self.SetSpawnPoint` (`self.GetTransform` _output_get_2))
  (`/Game/COMP2150/UI/UI_2150Gameplay.UpdateHealthBar` (`self.UI`) (`self.Health`) (`self.MaxHealth`))
  (`/Game/COMP2150/UI/UI_2150Gameplay.UpdateManaBar` (`self.UI`) (`self.Mana`) (`self.MaxMana`)))

(event `AddKey`
  (bind _returnvalue (+ (`self.Keys`) 1))
  ; Inventory
  (if (<= _returnvalue (`self.MaxKeys`))
    (set `self.Keys` _returnvalue)
    (`self.GameStateChange`)
    (`/Game/COMP2150/UI/UI_2150Gameplay.UpdateKeys` (`self.UI`) (`KismetStringLibrary.Conv_IntToString` (`self.Keys`)) (`KismetStringLibrary.Conv_IntToString` (`self.MaxKeys`)))
    (else
      (`KismetSystemLibrary.PrintString` "Max keys have been reached, but more keys have been placed." true true (struct :`R` 1.0 :`B` 0.00378 :`A` 1.0)))))

(event `UnlockBlink`
  ; UnlockingAbilities
  (set `self.BlinkUnlocked` true))

(event `UnlockShield`
  ; UnlockingAbilities
  (set `self.ShieldUnlocked` true))

(event `Respawn`
  (`self.K2_SetActorTransform` (`self.Player`) (`self.SpawnTransform`) false false)
  (set `self.Health` (`self.MaxHealth`))
  (set `self.Mana` (`self.MaxMana`))
  ; This is a bad way to do this and I feel bad.
  (set `/Game/COMP2150/Core/MainGame/BP_Sinead.State` "NewEnumerator0" (`self.Player`)))

(event `Reducehealth`
  (params (Damage :type Integer64))
  (set `self.Health` (`KismetMathLibrary.Conv_Int64ToInt` (- (`self.Health`) Damage)))
  (if (<= (`self.Health`) 0)
    (`self.Respawn`))
  (`/Game/COMP2150/UI/UI_2150Gameplay.UpdateHealthBar` (`self.UI`) (`self.Health`) (`self.MaxHealth`)))

(event `ReduceMana`
  (params (Cost :type Integer))
  (set `self.Mana` (- (`self.Mana`) Cost))
  (if (<= (`self.Mana`) 0.0)
    (set `self.Mana` 0.0))
  (`/Game/COMP2150/UI/UI_2150Gameplay.UpdateManaBar` (`self.UI`) (`self.Mana`) (`self.MaxMana`)))

(event `RestoreHealth`
  (params (Amount :type Integer))
  (set `self.Health` (`KismetMathLibrary.Conv_Int64ToInt` (+ (`self.Health`) Amount)))
  (if (>= (`self.Health`) (`self.MaxHealth`))
    (set `self.Health` (`self.MaxHealth`)))
  (`/Game/COMP2150/UI/UI_2150Gameplay.UpdateHealthBar` (`self.UI`) (`self.Health`) (`self.MaxHealth`)))

(event `RestoreMana`
  (if (< (`self.Mana`) (`self.MaxMana`))
    (bind _output_get (set `self.Mana` (+ (`self.Mana`) (`self.ManaRegen`))))
    (`/Game/COMP2150/UI/UI_2150Gameplay.UpdateManaBar` (`self.UI`) _output_get (`self.MaxMana`)))
  (`self.CheckCanBlink`)
  (`self.CheckCanShield`))

(event `SetSpawnPoint`
  (params (Input :type "Transform Structure"))
  (set `self.SpawnTransform` (`KismetMathLibrary.MakeTransform` (`KismetMathLibrary.MakeVector` (.x (.location Input)) (.y (.location Input)) (+ (.z (.location Input)) 200.0)) (.rotation Input))))

(event `CheckCanBlink`
  (bind _returnvalue (and (>= (`self.Mana`) (`/Game/COMP2150/Core/MainGame/BP_Sinead.BlinkCost` (`self.Player`))) (`self.BlinkUnlocked`)))
  (set `self.CanBlink` _returnvalue)
  (`/Game/COMP2150/UI/UI_2150Gameplay.UpdateBlinkIcon` (`self.UI`) _returnvalue))

(event `CheckCanShield`
  (bind _returnvalue (and (>= (`self.Mana`) (`/Game/COMP2150/Core/MainGame/BP_Sinead.ShieldCost` (`self.Player`))) (`self.ShieldUnlocked`)))
  (set `self.CanShield` _returnvalue)
  (`/Game/COMP2150/UI/UI_2150Gameplay.UpdateShieldIcon` (`self.UI`) _returnvalue))

(fn `UserConstructionScript`)