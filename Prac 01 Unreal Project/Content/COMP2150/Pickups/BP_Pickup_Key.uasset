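; BP_Pickup_Key is a key pickup that the player collects by walking into it.
; On BeginPlay it casts and caches the BP_2150GameMode.
; An overlap with an actor tagged Player calls AddKey on that game mode and destroys the pickup.
; The PickedUp event is present but empty.
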(event `self.ReceiveBeginPlay`
  (bind _asbp_2150game_mode (cast `/Game/COMP2150/Core/MainGame/BP_2150GameMode` (`GameplayStatics.GetGameMode`)))
  (set `self.GameMode` _asbp_2150game_mode))

(event `self.ReceiveActorBeginOverlap`
  (params (OtherActor :type "Actor Object Reference"))
  (if (`self.ActorHasTag` OtherActor "Player")
    (`/Game/COMP2150/Core/MainGame/BP_2150GameMode.AddKey` (`self.GameMode`))
    (`self.K2_DestroyActor`)))

(event `self.PickedUp`)

(fn `UserConstructionScript`
  (`parent.UserConstructionScript`))